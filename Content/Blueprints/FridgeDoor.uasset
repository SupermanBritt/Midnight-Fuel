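; Fridge door that swings open or shut each time its GrabComponent is grabbed.
; A Swing timeline drives the Door's relative yaw up to 90 degrees in the negative direction and stores its progress in CurrentValue.
; A zero CurrentValue plays the timeline forward, while any other value reverses it.
; The same Fridge_open sound plays attached to the Door on every toggle, including closing.
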(event `self.GrabComponent.OnGrabbed`
  (`self.Open/Close`))

(event `Open/Close`
  (`GameplayStatics.SpawnSoundAttached` "/Game/Sounds/Tooth_Guy/Fridge_open.Fridge_open" (`self.Door`) "None" (0.0 0.0 0.0) (struct) "KeepRelativeOffset" false 1.0 1.0 0.0 null null)
  (bind _output_get (set `self.Is Closed` (== (`self.Current Value`) 0.0)))
  (if _output_get
    (bind (_direction _swing_track) (`Timeline|Swing` :!label _label)
      (:`Update`
        (bind _output_get_2 (set `self.Current Value` _swing_track))
        (`SceneComponent.K2_SetRelativeRotation` (`self.Door`) (`KismetMathLibrary.MakeRotator` 0.0 0.0 (* _output_get_2 -90.0)) false false)))
    (else
      (goto _label :!via `Reverse`))))

(fn `UserConstructionScript`)