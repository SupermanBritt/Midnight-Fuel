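; VR grabbable pliers that pull a tooth from a mouth and respawn at their start transform on overlapping an OutOfBoundsBox.
; Grabbing enables input and adds the holding hand's weapon mapping context, which dropping removes.
; With InMouth set (toggled by MouthCheck), that hand's shoot press shows the held tooth, and release hides it and spawns a Tooth actor there.
; The pliers open on BeginPlay via their AnimBP; ClosedAnimation is never called here.
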(event `self.ReceiveBeginPlay`
  (set `self.OriginalPosition` (`self.GetTransform`))
  (`self.Open Animation`))

(event `Reset Position`
  (`self.K2_TeleportTo` (.location (`self.OriginalPosition`)) (.rotation (`self.OriginalPosition`))))

(event `self.Pliers.OnComponentBeginOverlap`
  (params (OverlappedComponent :type "PrimitiveComponent Object Reference") (OtherActor :type "Actor Object Reference") (OtherComp :type "PrimitiveComponent Object Reference") (OtherBodyIndex :type Integer) (bFromSweep :type Boolean) (SweepResult :type "HitResult Structure (by ref)"))
  (bind _returnvalue (`GameplayStatics.GetActorOfClass` "/Game/Blueprints/OutOfBoundsBox.OutOfBoundsBox_C"))
  (if (== (`GameplayStatics.GetObjectClass` _returnvalue) (`GameplayStatics.GetObjectClass` OtherActor))
    (`self.Reset Position`)))

(event `self.GrabComponent.OnGrabbed`
  (`self.EnableInput` (`GameplayStatics.GetPlayerController` 0))
  (`EnhancedInputSubsystemInterface.AddMappingContext` (pcsubsystem `EnhancedInputLocalPlayerSubsystem` (`GameplayStatics.GetPlayerController` 0)) (select `bool` (`|EnumEquality` (`/Game/VRTemplate/Blueprints/GrabComponent.GetHeldByHand` (`self.GrabComponent`)) "Right") :`false` "/Game/VRTemplate/Input/IMC_Weapon_Left.IMC_Weapon_Left" :`true` "/Game/VRTemplate/Input/IMC_Weapon_Right.IMC_Weapon_Right" :!type "InputMappingContext Object Reference") 1 (struct)))

(event `self.GrabComponent.OnDropped`
  (`self.DisableInput` (`GameplayStatics.GetPlayerController` 0))
  (`EnhancedInputSubsystemInterface.RemoveMappingContext` (pcsubsystem `EnhancedInputLocalPlayerSubsystem` (`GameplayStatics.GetPlayerController` 0)) (select `bool` (`|EnumEquality` (`/Game/VRTemplate/Blueprints/GrabComponent.GetHeldByHand` (`self.GrabComponent`)) "Right") :`false` "/Game/VRTemplate/Input/IMC_Weapon_Left.IMC_Weapon_Left" :`true` "/Game/VRTemplate/Input/IMC_Weapon_Right.IMC_Weapon_Right" :!type "InputMappingContext Object Reference") (struct)))

(event `EnhancedInput|/Game/VRTemplate/Input/Actions/IA_Shoot_Left`
  (params (ActionValue :type Boolean) (ElapsedSeconds :type "Float (double-precision)") (TriggeredSeconds :type "Float (double-precision)") (InputAction :type "InputAction Object Reference" :default "/Game/VRTemplate/Input/Actions/IA_Shoot_Left.IA_Shoot_Left"))
  (:`Started`
    (if (and (`|EnumEquality` (`/Game/VRTemplate/Blueprints/GrabComponent.GetHeldByHand` (`self.GrabComponent`)) "Left") (`self.InMouth`))
      (`SceneComponent.SetVisibility` (`self.Tooth`) true false)))
  (:`Completed`
    (if (`SceneComponent.IsVisible` (`self.Tooth`))
      (`SceneComponent.SetVisibility` (`self.Tooth`) false false)
      (`|SpawnActorFromClass` "/Game/Blueprints/Tooth.Tooth_C" (`SceneComponent.K2_GetComponentToWorld` (`self.Tooth`)) "Undefined" "MultiplyWithRoot" null null))))

(event `EnhancedInput|/Game/VRTemplate/Input/Actions/IA_Shoot_Right`
  (params (ActionValue :type Boolean) (ElapsedSeconds :type "Float (double-precision)") (TriggeredSeconds :type "Float (double-precision)") (InputAction :type "InputAction Object Reference" :default "/Game/VRTemplate/Input/Actions/IA_Shoot_Right.IA_Shoot_Right"))
  (:`Started`
    (if (and (`|EnumEquality` (`/Game/VRTemplate/Blueprints/GrabComponent.GetHeldByHand` (`self.GrabComponent`)) "Right") (`self.InMouth`))
      (`SceneComponent.SetVisibility` (`self.Tooth`) true false)))
  (:`Completed`
    (if (`SceneComponent.IsVisible` (`self.Tooth`))
      (`SceneComponent.SetVisibility` (`self.Tooth`) false false)
      (`|SpawnActorFromClass` "/Game/Blueprints/Tooth.Tooth_C" (`SceneComponent.K2_GetComponentToWorld` (`self.Tooth`)) "Undefined" "MultiplyWithRoot" null null))))

(event `Mouth Check`
  (if (== (`self.InMouth`) false)
    (set `self.InMouth` true)
    (else
      (set `self.InMouth` false))))

(fn `Closed Animation`
  (bind _aspliers_animation_blueprint (cast `/Game/Animations/Pliers/PliersAnimationBlueprint` (`SkeletalMeshComponent.GetAnimInstance` (`self.Pliers`))))
  (set `/Game/Animations/Pliers/PliersAnimationBlueprint.Is Closed` true _aspliers_animation_blueprint))

(fn `Open Animation`
  (bind _aspliers_animation_blueprint (cast `/Game/Animations/Pliers/PliersAnimationBlueprint` (`SkeletalMeshComponent.GetAnimInstance` (`self.Pliers`))))
  (set `/Game/Animations/Pliers/PliersAnimationBlueprint.Is Closed` false _aspliers_animation_blueprint))

(fn `UserConstructionScript`)