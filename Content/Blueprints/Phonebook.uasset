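; Physics-simulated phonebook actor for a VR game that can be delivered to progress a PhoneGuy sequence.
; It caches its starting transform on BeginPlay and returns there, briefly disabling physics, when it overlaps the OutOfBoundsBox.
; Deliver acts only once the VRPawn's AudioFinished flag is set: it spawns a Key at the original transform, sends PhoneGuy to the car and destroys the phonebook.
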(event `self.ReceiveBeginPlay`
  (set `self.OriginalPosition` (`self.GetTransform`)))

(event `Reset Position`
  (`PrimitiveComponent.SetSimulatePhysics` (`self.Phonebook`) false)
  (`self.K2_SetActorTransform` (`self.OriginalPosition`))
  (`PrimitiveComponent.SetSimulatePhysics` (`self.Phonebook`) true))

(event `self.Phonebook.OnComponentBeginOverlap`
  (params (OverlappedComponent :type "PrimitiveComponent Object Reference") (OtherActor :type "Actor Object Reference") (OtherComp :type "PrimitiveComponent Object Reference") (OtherBodyIndex :type Integer) (bFromSweep :type Boolean) (SweepResult :type "HitResult Structure (by ref)"))
  (bind _returnvalue (`GameplayStatics.GetActorOfClass` "/Game/Blueprints/OutOfBoundsBox.OutOfBoundsBox_C"))
  (if (== _returnvalue OtherActor)
    (`self.Reset Position`)))

(event `Deliver`
  (bind _returnvalue (`GameplayStatics.GetActorOfClass` "/Game/VRTemplate/Blueprints/VRPawn.VRPawn_C"))
  (if (`/Game/VRTemplate/Blueprints/VRPawn.AudioFinished` _returnvalue)
    (`|SpawnActorFromClass` "/Game/Blueprints/Key.Key_C" (`self.OriginalPosition`) "Undefined" "MultiplyWithRoot" null null)
    (bind _returnvalue_2 (`GameplayStatics.GetActorOfClass` "/Game/Blueprints/PhoneGuy.PhoneGuy_C"))
    (`/Game/Blueprints/PhoneGuy.Get In Car` _returnvalue_2)
    (`self.K2_DestroyActor`)))

(fn `UserConstructionScript`)