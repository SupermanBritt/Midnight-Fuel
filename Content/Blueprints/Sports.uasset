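; Sports car Blueprint that drives along scripted spline paths into and out of a gas station.
; MoveToGasStation and MoveAwayFromGasStation each run a Timeline that lerps distance along their path spline, setting the actor's location and rotation.
; Attached engine sounds play per move, with the arrival sound fading out on completion.
; Two rect lights switch on when moving and off after arrival.
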(event `MoveToGasStation`
  (`self.Turn On Lights`)
  (bind _returnvalue (`GameplayStatics.SpawnSoundAttached` "/Game/Sounds/CarSounds/CarEnterCue.CarEnterCue" (`self.Hatchback_Audio`) "None" (0.0 0.0 0.0) (struct) "KeepRelativeOffset" false 1.0 1.0 0.0 null null))
  (bind (_direction _alpha) (`Timeline|Timeline`)
    (:`Update`
      (`self.K2_SetActorLocationAndRotation` (.location (`SplineComponent.GetTransformAtDistanceAlongSpline` (`/Game/Blueprints/PickupPath.Spline` (`self.PathToGasStation`)) (`KismetMathLibrary.Lerp` 0.0 (`SplineComponent.GetSplineLength` (`/Game/Blueprints/PickupPath.Spline` (`self.PathToGasStation`))) _alpha) "World" false)) (.rotation (`SplineComponent.GetTransformAtDistanceAlongSpline` (`/Game/Blueprints/PickupPath.Spline` (`self.PathToGasStation`)) (`KismetMathLibrary.Lerp` 0.0 (`SplineComponent.GetSplineLength` (`/Game/Blueprints/PickupPath.Spline` (`self.PathToGasStation`))) _alpha) "World" false))))
    (:`Finished`
      (`AudioComponent.FadeOut` _returnvalue 0.5 0.0 "Linear")
      (`self.Turn Off Lights`))))

(event `MoveAwayFromGasStation`
  (`GameplayStatics.SpawnSoundAttached` "/Game/Sounds/CarSounds/CarStart.CarStart" (`self.Hatchback_Audio`) "None" (0.0 0.0 0.0) (struct) "KeepRelativeOffset" false 1.0 1.0 0.0 null null)
  (`GameplayStatics.SpawnSoundAttached` "/Game/Sounds/CarSounds/CarLeaveCue.CarLeaveCue" (`self.Hatchback_Audio`) "None" (0.0 0.0 0.0) (struct) "KeepRelativeOffset" false 1.0 1.0 0.0 null null)
  (`self.Turn On Lights`)
  (bind (_direction _alpha) (`Timeline|Timeline_0`)
    (:`Update`
      (`self.K2_SetActorLocationAndRotation` (.location (`SplineComponent.GetTransformAtDistanceAlongSpline` (`/Game/Blueprints/PickupPath.Spline` (`self.PathAwayFromGasStation`)) (`KismetMathLibrary.Lerp` 0.0 (`SplineComponent.GetSplineLength` (`/Game/Blueprints/PickupPath.Spline` (`self.PathAwayFromGasStation`))) _alpha) "World" false)) (.rotation (`SplineComponent.GetTransformAtDistanceAlongSpline` (`/Game/Blueprints/PickupPath.Spline` (`self.PathAwayFromGasStation`)) (`KismetMathLibrary.Lerp` 0.0 (`SplineComponent.GetSplineLength` (`/Game/Blueprints/PickupPath.Spline` (`self.PathAwayFromGasStation`))) _alpha) "World" false))))))

(fn `Turn Off Lights`
  (`SceneComponent.SetVisibility` (`self.RectLight`) false false)
  (`SceneComponent.SetVisibility` (`self.RectLight1`) false false))

(fn `Turn On Lights`
  (`SceneComponent.SetVisibility` (`self.RectLight`) true false)
  (`SceneComponent.SetVisibility` (`self.RectLight1`) true false))

(fn `UserConstructionScript`)