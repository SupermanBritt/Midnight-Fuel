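; Scripted old-man customer NPC that leaves a car, walks to a service window and later returns to the car.
; GetOutofCar plays the exit animation, moves it along the CustomerPath spline by timeline, then voices a line before setting AtWindow.
; GetInCar plays a farewell, walks the spline back with yaw flipped, enters the car, resets position and calls CallThirdCustomer.
; Helpers toggle AnimBP flags; body parts follow Body via leader pose.
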(event `self.ReceiveBeginPlay`
  (set `self.Original Position` (`self.K2_GetActorLocation`))
  (bind _returnvalue (`GameplayStatics.GetActorOfClass` "/Game/Blueprints/CustomerPath.CustomerPath_C"))
  (set `self.Customer Path` _returnvalue))

(event `Get Out of Car`
  (`self.K2_TeleportTo` (`KismetMathLibrary.MakeVector` (+ (.x (.location (`SplineComponent.GetTransformAtDistanceAlongSpline` (`/Game/Blueprints/CustomerPath.Spline` (`self.Customer Path`)) (`KismetMathLibrary.Lerp` 0.0 (`SplineComponent.GetSplineLength` (`/Game/Blueprints/CustomerPath.Spline` (`self.Customer Path`)))) "World" false))) -80.0) (+ (.y (.location (`SplineComponent.GetTransformAtDistanceAlongSpline` (`/Game/Blueprints/CustomerPath.Spline` (`self.Customer Path`)) (`KismetMathLibrary.Lerp` 0.0 (`SplineComponent.GetSplineLength` (`/Game/Blueprints/CustomerPath.Spline` (`self.Customer Path`)))) "World" false))) 80.0) (.z (.location (`SplineComponent.GetTransformAtDistanceAlongSpline` (`/Game/Blueprints/CustomerPath.Spline` (`self.Customer Path`)) (`KismetMathLibrary.Lerp` 0.0 (`SplineComponent.GetSplineLength` (`/Game/Blueprints/CustomerPath.Spline` (`self.Customer Path`)))) "World" false)))) (struct :`Yaw` 50.0))
  (`self.ExitCarAnimation`)
  (`KismetSystemLibrary.Delay` (`AnimSequenceBase.SequenceLength` (`self.ExitCarAnimationRef`)))
  (`self.Walk Animation`)
  (bind (_direction _alpha) (`Timeline|Timeline`)
    (:`Update`
      (`self.K2_SetActorLocationAndRotation` (.location (`SplineComponent.GetTransformAtDistanceAlongSpline` (`/Game/Blueprints/CustomerPath.Spline` (`self.Customer Path`)) (`KismetMathLibrary.Lerp` 0.0 (`SplineComponent.GetSplineLength` (`/Game/Blueprints/CustomerPath.Spline` (`self.Customer Path`))) _alpha) "World" false)) (.rotation (`SplineComponent.GetTransformAtDistanceAlongSpline` (`/Game/Blueprints/CustomerPath.Spline` (`self.Customer Path`)) (`KismetMathLibrary.Lerp` 0.0 (`SplineComponent.GetSplineLength` (`/Game/Blueprints/CustomerPath.Spline` (`self.Customer Path`))) _alpha) "World" false))))
    (:`Finished`
      (`self.IdleAnimation`)
      (bind _returnvalue (`GameplayStatics.SpawnSoundAttached` "/Game/Sounds/Customer_Sounds/Old_Man_Voice_Enter.Old_Man_Voice_Enter" (`self.Mesh`) "None" (0.0 0.0 0.0) (struct) "KeepRelativeOffset" false 1.0 1.0 0.0 "/Game/Sounds/Phone_Guy/PhoneGuyAttenuation.PhoneGuyAttenuation" null))
      (add `AudioComponent.OnAudioFinished` _returnvalue (delegate `Item Asking Audio Done`)))))

(event `Item Asking Audio Done`
  (set `self.At Window` true))

(event `Get In Car`
  (bind _returnvalue (`GameplayStatics.SpawnSoundAttached` "/Game/Sounds/Customer_Sounds/Old_Man_Voice_Leave.Old_Man_Voice_Leave" (`self.Mesh`) "None" (0.0 0.0 0.0) (struct) "KeepRelativeOffset" false 1.0 1.0 0.0 "/Game/Sounds/Phone_Guy/PhoneGuyAttenuation.PhoneGuyAttenuation" null))
  (add `AudioComponent.OnAudioFinished` _returnvalue (delegate `Thank You Done`)))

(event `Thank You Done`
  (`self.Walk Animation`)
  (bind (_direction _alpha) (`Timeline|Timeline_0` :!via `ReverseFromEnd`)
    (:`Update`
      (`self.K2_SetActorLocationAndRotation` (.location (`SplineComponent.GetTransformAtDistanceAlongSpline` (`/Game/Blueprints/CustomerPath.Spline` (`self.Customer Path`)) (`KismetMathLibrary.Lerp` 0.0 (`SplineComponent.GetSplineLength` (`/Game/Blueprints/CustomerPath.Spline` (`self.Customer Path`))) _alpha) "World" false)) (`KismetMathLibrary.MakeRotator` (.roll (.rotation (`SplineComponent.GetTransformAtDistanceAlongSpline` (`/Game/Blueprints/CustomerPath.Spline` (`self.Customer Path`)) (`KismetMathLibrary.Lerp` 0.0 (`SplineComponent.GetSplineLength` (`/Game/Blueprints/CustomerPath.Spline` (`self.Customer Path`))) _alpha) "World" false))) (.pitch (.rotation (`SplineComponent.GetTransformAtDistanceAlongSpline` (`/Game/Blueprints/CustomerPath.Spline` (`self.Customer Path`)) (`KismetMathLibrary.Lerp` 0.0 (`SplineComponent.GetSplineLength` (`/Game/Blueprints/CustomerPath.Spline` (`self.Customer Path`))) _alpha) "World" false))) (+ (.yaw (.rotation (`SplineComponent.GetTransformAtDistanceAlongSpline` (`/Game/Blueprints/CustomerPath.Spline` (`self.Customer Path`)) (`KismetMathLibrary.Lerp` 0.0 (`SplineComponent.GetSplineLength` (`/Game/Blueprints/CustomerPath.Spline` (`self.Customer Path`))) _alpha) "World" false))) 180.0))))
    (:`Finished`
      (`self.GetInCarAnimation`)
      (`KismetSystemLibrary.Delay` (`AnimSequenceBase.SequenceLength` (`self.EnterCarAnimationRef`)))
      (`self.K2_TeleportTo` (`self.Original Position`))
      (`self.Third Customer`))))

(fn `ExitCarAnimation`
  (bind _asmanny_animation_blueprint (cast `/Game/Animations/MannyAnimationBlueprint` (`SkeletalMeshComponent.GetAnimInstance` (`self.Mesh`))))
  (set `/Game/Animations/MannyAnimationBlueprint.IsWalking` false _asmanny_animation_blueprint)
  (set `/Game/Animations/MannyAnimationBlueprint.GetInCar` false _asmanny_animation_blueprint)
  (set `/Game/Animations/MannyAnimationBlueprint.ExitCar` true _asmanny_animation_blueprint))

(fn `GetInCarAnimation`
  (bind _asmanny_animation_blueprint (cast `/Game/Animations/MannyAnimationBlueprint` (`SkeletalMeshComponent.GetAnimInstance` (`self.Mesh`))))
  (set `/Game/Animations/MannyAnimationBlueprint.IsWalking` false _asmanny_animation_blueprint)
  (set `/Game/Animations/MannyAnimationBlueprint.GetInCar` true _asmanny_animation_blueprint)
  (set `/Game/Animations/MannyAnimationBlueprint.ExitCar` false _asmanny_animation_blueprint))

(fn `IdleAnimation`
  (bind _asmanny_animation_blueprint (cast `/Game/Animations/MannyAnimationBlueprint` (`SkeletalMeshComponent.GetAnimInstance` (`self.Mesh`))))
  (set `/Game/Animations/MannyAnimationBlueprint.IsWalking` false _asmanny_animation_blueprint)
  (set `/Game/Animations/MannyAnimationBlueprint.GetInCar` false _asmanny_animation_blueprint)
  (set `/Game/Animations/MannyAnimationBlueprint.ExitCar` false _asmanny_animation_blueprint))

(fn `UserConstructionScript`
  (`SkinnedMeshComponent.SetLeaderPoseComponent` (`self.Legs`) (`self.Body`) false false)
  (`SkinnedMeshComponent.SetLeaderPoseComponent` (`self.Feet`) (`self.Body`) false false)
  (`SkinnedMeshComponent.SetLeaderPoseComponent` (`self.Face`) (`self.Body`) false false)
  (`SkinnedMeshComponent.SetLeaderPoseComponent` (`self.Torso`) (`self.Body`) false false))

(fn `Walk Animation`
  (bind _asmanny_animation_blueprint (cast `/Game/Animations/MannyAnimationBlueprint` (`SkeletalMeshComponent.GetAnimInstance` (`self.Mesh`))))
  (set `/Game/Animations/MannyAnimationBlueprint.IsWalking` true _asmanny_animation_blueprint)
  (set `/Game/Animations/MannyAnimationBlueprint.GetInCar` false _asmanny_animation_blueprint)
  (set `/Game/Animations/MannyAnimationBlueprint.ExitCar` false _asmanny_animation_blueprint))