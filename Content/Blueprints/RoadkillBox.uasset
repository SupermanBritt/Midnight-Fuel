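; RoadkillBox is an overlap actor apparently meant to make the VR player roadkill, but its overlap event is empty.
; BeginPlay caches the NotTeleportZone actor's transform.
; Disconnected logic would match "VRPawn" by name prefix, restore that zone, call MakePlayerRoadkill on the SUV, delay, play then immediately pause MainSequence, and quit.
; As wired, only the transform caching runs.
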(event `self.ReceiveBeginPlay`
  (set `self.OriginalNoTeleportZoneTransform` (`self.GetTransform` (`self.NotTeleportZone`))))

(event `self.ReceiveActorBeginOverlap`
  (params (OtherActor :type "Actor Object Reference")))

(fn `UserConstructionScript`)