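; Chips is a physics-simulated item that can be delivered to a customer at the window.
; It stores its starting transform at BeginPlay and returns there, briefly disabling physics, when its mesh overlaps an actor of the OutOfBoundsBox class.
; Deliver looks up the NormalCustomer1 actor by class and, if that customer is at the window, calls its GetInCar and destroys the chips.
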(event `self.ReceiveBeginPlay`
  (set `self.Original Position` (`self.GetTransform`)))

(event `Reset Position`
  (bind _chips (`self.Chips`))
  (`PrimitiveComponent.SetSimulatePhysics` _chips false)
  (`self.K2_SetActorTransform` (`self.Original Position`))
  (`PrimitiveComponent.SetSimulatePhysics` _chips true))

(event `self.Chips.OnComponentBeginOverlap`
  (params (OverlappedComponent :type "PrimitiveComponent Object Reference") (OtherActor :type "Actor Object Reference") (OtherComp :type "PrimitiveComponent Object Reference") (OtherBodyIndex :type Integer) (bFromSweep :type Boolean) (SweepResult :type "HitResult Structure (by ref)"))
  (bind _returnvalue (`GameplayStatics.GetActorOfClass` "/Game/Blueprints/OutOfBoundsBox.OutOfBoundsBox_C"))
  (if (== (`GameplayStatics.GetObjectClass` _returnvalue) (`GameplayStatics.GetObjectClass` OtherActor))
    (`self.Reset Position`)))

(event `Deliver`
  (bind _returnvalue (`GameplayStatics.GetActorOfClass` "/Game/Blueprints/NormalCustomer1.NormalCustomer1_C"))
  (if (`/Game/Blueprints/NormalCustomer1.AtWindow` _returnvalue)
    (`/Game/Blueprints/NormalCustomer1.Get In Car` _returnvalue)
    (`self.K2_DestroyActor`)))

(fn `UserConstructionScript`)