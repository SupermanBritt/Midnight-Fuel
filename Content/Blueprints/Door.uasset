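; Locked door actor that opens when a component named Key overlaps its Box, destroying that key's actor and showing its own Key mesh.
; Once unlocked, Tick lowers the yaw one degree per frame to 45, then plays MainSequence in reverse and quits the game after a short delay.
; Grabbing the door immediately attempts a release and plays the Door_locking sound at the Key's location.
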(event `self.ReceiveTick`
  (params (DeltaSeconds :type "Float (single-precision)"))
  (bind _angle (`self.Angle`))
  (bind _returnvalue (- _angle 1.0))
  (if (and (`self.Unlocked`) (> _angle 45.0))
    (bind _output_get (set `self.Angle` _returnvalue))
    (`self.K2_SetActorRotation` (`KismetMathLibrary.MakeRotator` 0.0 0.0 _output_get))
    (elif (== _angle 45.0)
      (set `self.Angle` _returnvalue)
      (bind _outactor (`LevelSequencePlayer.CreateLevelSequencePlayer` "/Game/Maps/MainSequence.MainSequence"))
      (`MovieSceneSequencePlayer.PlayReverse` (`LevelSequenceActor.SequencePlayer` _outactor))
      (`KismetSystemLibrary.Delay` 2.0)
      (`KismetSystemLibrary.QuitGame` null "Quit"))))

(event `self.Box.OnComponentBeginOverlap`
  (params (OverlappedComponent :type "PrimitiveComponent Object Reference") (OtherActor :type "Actor Object Reference") (OtherComp :type "PrimitiveComponent Object Reference") (OtherBodyIndex :type Integer) (bFromSweep :type Boolean) (SweepResult :type "HitResult Structure (by ref)"))
  (if (`KismetStringLibrary.EqualEqual_StrStr` (`KismetSystemLibrary.GetObjectName` OtherComp) "Key")
    (set `self.Unlocked` true)
    (`self.K2_DestroyActor` OtherActor)
    (`SceneComponent.SetVisibility` (`self.Key`) true false)))

(event `self.GrabComponent.OnGrabbed`
  (`/Game/VRTemplate/Blueprints/GrabComponent.TryRelease` (`self.GrabComponent`))
  (`GameplayStatics.PlaySoundAtLocation` "/Game/Sounds/Door_locking.Door_locking" (`SceneComponent.K2_GetComponentLocation` (`self.Key`)) (struct) 1.0 1.0 0.0 null null null null))

(fn `UserConstructionScript`)