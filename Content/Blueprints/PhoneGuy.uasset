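; PhoneGuy is the VR horror antagonist who arrives at the gas station by car, later returns asking for pliers, and can stab the player into game over.
; While the player lacks the phone, a recursive delay loop teleports him through preset spots, raising unhappiness until he kills.
; The kill places him ahead of or behind the player's camera; from behind, he waits until they turn around.
; Scripted sequences drive anim-instance flags, while a timeline blends randomized morph-target expressions.
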(event `StartTeleporting`
  (`KismetSystemLibrary.Delay` 7.0)
  (if (`self.ShouldTeleport`)
    (if (<= (+ (`self.LocationsIndex`) 1) 3)
      (switch `int` (`self.LocationsIndex`)
        (:`0`
          (`self.At Location 2`)
          (`self.K2_TeleportTo` (`KismetMathLibrary.TransformLocation` (`self.StartingPosition`) (`self.Location1`))))
        (:`1`
          (`self.At Location 3`)
          (`self.K2_TeleportTo` (`KismetMathLibrary.TransformLocation` (`self.StartingPosition`) (`self.Location2`))))
        (:`2`
          (`self.At Location 4`)
          (`self.K2_TeleportTo` (`KismetMathLibrary.TransformLocation` (`self.StartingPosition`) (`self.Location3`)))))
      (`self.Increase Unhappiness`)
      (set `self.LocationsIndex` (+ (`self.LocationsIndex`) 1))
      (`self.StartTeleporting`)
      (else
        (`self.Kill`)))
    (else
      (`self.StartTeleporting`))))

(event `Kill`
  (set `self.PhoneLinesActivated` false)
  (`self.K2_SetActorTransform` (`self.NotTeleportZone`) (`KismetMathLibrary.MakeTransform` (+ (.location (`self.GetTransform` (`self.NotTeleportZone`))) (0.0 5000.0 0.0)) (.rotation (`self.GetTransform` (`self.NotTeleportZone`))) (.scale (`self.GetTransform` (`self.NotTeleportZone`)))) false false)
  (`self.At Kill Location`)
  (`self.Unhinged Malice`)
  (bind _returnvalue (`GameplayStatics.GetActorOfClass` "/Game/VRTemplate/Blueprints/VRPawn.VRPawn_C"))
  (bind _x (.x (.location (`SceneComponent.K2_GetComponentToWorld` (`/Game/VRTemplate/Blueprints/VRPawn.Camera` _returnvalue)))))
  (bind _y (.y (.location (`SceneComponent.K2_GetComponentToWorld` (`/Game/VRTemplate/Blueprints/VRPawn.Camera` _returnvalue)))))
  (if (>= _x -9900.0)
    (`self.K2_SetActorTransform` (`KismetMathLibrary.MakeTransform` (`KismetMathLibrary.MakeVector` (+ _x -160.0) _y 91.0))) ; Teleports In Front of the player
    (`self.Stab`)
    (else
      (`self.K2_SetActorTransform` (`KismetMathLibrary.MakeTransform` (`KismetMathLibrary.MakeVector` (+ _x 160.0) _y 91.0) (struct :`Yaw` 180.0))) ; Teleports Behind the player
      (set `self.ReadyToKill` true))))

(event `Stab`
  (`self.Stabbing Animation`)
  (`KismetSystemLibrary.Delay` (`AnimSequenceBase.SequenceLength` (`self.StabbingAnimationReference`)))
  (`GameplayStatics.OpenLevel` "GameOverMenu"))

(event `Get In Car`
  (`self.K2_TeleportTo` (`KismetMathLibrary.TransformLocation` (`self.StartingPosition`) (`self.WindowLocation`)))
  (`self.Grabbing Item Animation`)
  (`KismetSystemLibrary.Delay` (`AnimSequenceBase.SequenceLength` (`self.GrabbingItemAnimationReference`)))
  (`self.Staring Animation`)
  (`self.Unhinged Smile`)
  (`KismetSystemLibrary.Delay` 3.0)
  (`self.K2_TeleportTo` (`KismetMathLibrary.TransformLocation` (`self.StartingPosition`) (`self.LocationGetInCar`)) (struct :`Yaw` 90.0))
  (`self.GetInCarAnimation`)
  (`KismetSystemLibrary.Delay` (`AnimSequenceBase.SequenceLength` (`self.EnterCarAnimationRef`)))
  (`self.K2_TeleportTo` (`KismetMathLibrary.TransformLocation` (`self.StartingPosition`)))
  (`KismetSystemLibrary.Delay` 3.0)
  (`/Game/Blueprints/SUV.MoveAwayFromGasStation` (`self.Car`))
  (set `self.TurnLightsBackOn` true)
  (set `self.Mistakes` 0)
  (set `self.PhoneLinesActivated` false)
  (`self.Phone Guy Gone`))

(event `self.ReceiveTick`
  (params (DeltaSeconds :type "Float (single-precision)"))
  (bind _returnvalue (`GameplayStatics.GetActorOfClass` "/Game/VRTemplate/Blueprints/VRPawn.VRPawn_C"))
  (if (`self.ReadyToKill`)
    (bind _yaw (.yaw (`SceneComponent.K2_GetComponentRotation` (`/Game/VRTemplate/Blueprints/VRPawn.Camera` _returnvalue))))
    (if (and (<= _yaw 25.0) (>= _yaw -25.0))
      (`self.Stab`))
    (else
      (if (`/Game/VRTemplate/Blueprints/VRPawn.HasPhone` _returnvalue)
        (set `self.ShouldTeleport` false :!label _label)
        (elif (`/Game/VRTemplate/Blueprints/VRPawn.AudioFinished` _returnvalue)
          (goto _label)
          (else
            (set `self.ShouldTeleport` true))))
      (bind _returnvalue_2 (`GameplayStatics.GetActorOfClass` "/Game/Blueprints/Pliers.Pliers_C"))
      (if (`/Game/Blueprints/Pliers.PhoneGuyWaiting` _returnvalue_2)
        (bind (_returnvalue_roll _returnvalue_pitch _returnvalue_yaw) (`KismetMathLibrary.BreakRotator` (`KismetMathLibrary.FindLookAtRotation` (`self.K2_GetActorLocation`) (`self.K2_GetActorLocation` _returnvalue))))
        (set `self.Head Rotation` _returnvalue_yaw)
        (`self.Staring Animation`)))))

(event `Get Out Of Car`
  (`self.K2_TeleportTo` (`KismetMathLibrary.TransformLocation` (`self.StartingPosition`) (`self.LocationExitCarAnimation`)))
  (`self.ExitCarAnimation`)
  (`KismetSystemLibrary.Delay` (`AnimSequenceBase.SequenceLength` (`self.ExitCarAnimationRef`)))
  (`self.K2_TeleportTo` (`KismetMathLibrary.TransformLocation` (`self.StartingPosition`) (`self.Location 0`)))
  (`self.At Location 1`)
  (`self.Phone Guy Out of Car`)
  (`self.Staring Animation`)
  (set `self.PhoneLinesActivated` true)
  (`self.StartTeleporting`))

(event `Make Final Call`
  (set `self.ToothLinesActivated` true)
  (bind _returnvalue (`GameplayStatics.GetActorOfClass` "/Game/Blueprints/FridgeDoor.FridgeDoor_C"))
  (if (`/Game/Blueprints/FridgeDoor.Is Closed` _returnvalue)
    (`/Game/Blueprints/FridgeDoor.Open/Close` _returnvalue))
  (`|SpawnActorFromClass` "/Game/Blueprints/DecapitatedHead.DecapitatedHead_C" (`KismetMathLibrary.MakeTransform` (-10075.0 10300.0 104.0) (struct :`Roll` -25.0)) "Undefined" "MultiplyWithRoot" null null))

(event `self.ReceiveBeginPlay`
  (set `self.Locations` (`|MakeArray` (`self.Location1`) (`self.Location2`) (`self.Location3`)))
  (set `self.StartingPosition` (`self.GetTransform`)))

(event `Get Out Again`
  (`self.K2_TeleportTo` (`KismetMathLibrary.TransformLocation` (`self.StartingPosition`) (`self.LocationExitCarAnimation`)))
  (`self.ExitCarAnimation`)
  (`KismetSystemLibrary.Delay` (`AnimSequenceBase.SequenceLength` (`self.ExitCarAnimationRef`)))
  (`self.K2_TeleportTo` (`KismetMathLibrary.TransformLocation` (`self.StartingPosition`) (`self.Location 0`)))
  (set `self.TurnLightsBackOn` false)
  (`self.Phone Guy Out Again`)
  (`self.Staring Animation`)
  (`KismetSystemLibrary.Delay` 2.0)
  (`self.K2_TeleportTo` (`KismetMathLibrary.TransformLocation` (`self.StartingPosition`) (`self.WindowLocation`)))
  (`self.Smile`)
  (bind _returnvalue (`GameplayStatics.SpawnSoundAttached` "/Game/Sounds/Tooth_Guy/Tooth_Guy_Ask_Normalized.Tooth_Guy_Ask_Normalized" (`self.Mesh`) "None" (0.0 0.0 0.0) (struct) "KeepRelativeOffset" false 1.0 1.0 0.0 "/Game/Sounds/Phone_Guy/PhoneGuyAttenuation.PhoneGuyAttenuation" null))
  (add `AudioComponent.OnAudioFinished` _returnvalue (delegate `Give Pliers`)))

(event `Get In Again`
  (`self.Grabbing Item Animation`)
  (`KismetSystemLibrary.Delay` (`AnimSequenceBase.SequenceLength` (`self.GrabbingItemAnimationReference`)))
  (`self.Staring Animation`)
  (`self.Unhinged Smile`)
  (bind _returnvalue (`GameplayStatics.SpawnSoundAttached` "/Game/Sounds/Tooth_Guy/Tooth_Guy_Thank_Normalized.Tooth_Guy_Thank_Normalized" (`self.Mesh`) "None" (0.0 0.0 0.0) (struct) "KeepRelativeOffset" false 1.0 1.0 0.0 "/Game/Sounds/Phone_Guy/PhoneGuyAttenuation.PhoneGuyAttenuation" null))
  (add `AudioComponent.OnAudioFinished` _returnvalue (delegate `Keep Leaving`)))

(event `Give Pliers`
  (bind _returnvalue (`GameplayStatics.GetActorOfClass` "/Game/Blueprints/Tray.Tray_C"))
  (`/Game/Blueprints/Tray.Pull Tray Out` _returnvalue)
  (`KismetSystemLibrary.Delay` 1.5)
  ;[1 1 1] Make pliers spawn in here
  (bind _returnvalue_2 (`GameplayStatics.GetActorOfClass` "/Game/Blueprints/Pliers.Pliers_C"))
  (set `/Game/Blueprints/Pliers.PhoneGuyWaiting` true _returnvalue_2))

(event `Keep Leaving`
  (`self.K2_TeleportTo` (`KismetMathLibrary.TransformLocation` (`self.StartingPosition`) (`self.LocationGetInCar`)) (struct :`Yaw` 90.0))
  (`self.GetInCarAnimation`)
  (`KismetSystemLibrary.Delay` (`AnimSequenceBase.SequenceLength` (`self.EnterCarAnimationRef`)))
  (`self.K2_TeleportTo` (`KismetMathLibrary.TransformLocation` (`self.StartingPosition`)))
  (`KismetSystemLibrary.Delay` 3.0)
  (`/Game/Blueprints/SUV.MoveAwayFromGasStation` (`self.Car`))
  (set `self.TurnLightsBackOn` true)
  (`self.Phone Guy Gone Again`))

(event `Increase Unhappiness`
  (bind _output_get (set `self.Mistakes` (+ (`self.Mistakes`) 1)))
  (switch `int` _output_get
    (:`1`
      (`self.Uneven Frown`))
    (:`2`
      (`self.Uneasy Frown`))
    (:`3`
      (`self.Unhinged Frown`))
    (:`4`
      (`self.Unsafe Frown`))
    (:`5`
      (`self.Kill`))))

(event `Smile`
  (`self.Morph Target Animations` 0.0 0.0 0.0 0.0 0.0 0.0 0.0 0.0 0.0 0.0 0.7 0.5)
  (`KismetSystemLibrary.Delay` 2.5))

(event `Uneven Smile`
  (`self.Morph Target Animations` 0.0 0.0 0.0 0.0 0.0 0.0 0.0 0.35 0.35 0.0 0.45 0.2)
  (`KismetSystemLibrary.Delay` 2.5))

(event `Unhinged Smile`
  (`self.Morph Target Animations` 0.0 0.0 0.0 0.0 0.0 0.0 0.8 0.0 0.7 0.0 0.0 0.0 0.0 0.0 0.05)
  (`KismetSystemLibrary.Delay` 2.5))

(event `Frown`
  (`self.Morph Target Animations` 0.0 0.0 0.0 0.0 0.0 0.1 0.0 0.0 0.0 0.0 0.0 0.0 0.0 0.0 0.1)
  (`KismetSystemLibrary.Delay` 2.5))

(event `Uneven Frown`
  (`self.Morph Target Animations` 0.4 0.4 0.0 0.0 0.0 0.3 0.0 0.35 0.0 0.3)
  (`KismetSystemLibrary.Delay` 2.5))

(event `Uneasy Frown`
  (`self.Morph Target Animations` 0.6 0.6 0.0 0.0 0.0 0.15 0.4 0.2 0.0 0.45)
  (`KismetSystemLibrary.Delay` 2.5))

(event `Unhinged Frown`
  (`self.Morph Target Animations` 0.75 0.8 0.0 0.0 0.0 0.0 0.8 0.0 0.0 0.65)
  (`KismetSystemLibrary.Delay` 2.5))

(event `Unsafe Frown`
  (`self.Morph Target Animations` 1.0 1.0 0.0 0.0 0.0 0.0 0.9 0.3 0.0 0.3 0.0 0.0 0.0 0.0 0.25)
  (`KismetSystemLibrary.Delay` 2.5))

(event `Malice`
  (`self.Morph Target Animations` 0.7 0.7 0.0 0.0 0.0 0.0 0.6 0.75 0.4)
  (`KismetSystemLibrary.Delay` 2.5))

(event `Unhinged Malice`
  (`self.Morph Target Animations` 1.0 1.0 0.0 0.0 0.0 0.0 1.0 0.6 0.0 0.0 0.0 0.0 0.0 0.0 0.5)
  (`KismetSystemLibrary.Delay` 2.5))

(event `Morph Target Animations`
  (params (Vinny_LeftBrow_Mad :type "Float (double-precision)") (Vinny_RightBrow_Mad :type "Float (double-precision)") (Vinny_LeftBrow_Sad :type "Float (double-precision)") (Vinny_RightBrow_Sad :type "Float (double-precision)") (Vinny_Mouth_Smile :type "Float (double-precision)") (Vinny_Mouth_Frown :type "Float (double-precision)") (Vinny_Infection :type "Float (double-precision)") (Vinny_Creep :type "Float (double-precision)") (Toothy_Smile :type "Float (double-precision)") (Tooth_Scowl :type "Float (double-precision)") (Right_Smirk :type "Float (double-precision)") (Left_Smirk :type "Float (double-precision)") (Right_Eye_Wide :type "Float (double-precision)") (Left_Eye_Wide :type "Float (double-precision)") (Melt :type "Float (double-precision)"))
  (bind (_direction _alpha) (`Timeline|Timeline_Morph` :!via `PlayFromStart`)
    (:`Update`
      (set `self.Alpha` _alpha)
      (`SkeletalMeshComponent.SetMorphTarget` (`self.Face`) "Vinny_LeftBrow_Mad" (`KismetMathLibrary.Lerp` (`SkeletalMeshComponent.GetMorphTarget` (`self.Face`) "Vinny_LeftBrow_Mad") (+ Vinny_LeftBrow_Mad (`KismetMathLibrary.RandomFloatInRange` -0.1 0.1)) (`self.Alpha`)) true)
      (`SkeletalMeshComponent.SetMorphTarget` (`self.Face`) "Vinny_RightBrow_Mad" (`KismetMathLibrary.Lerp` (`SkeletalMeshComponent.GetMorphTarget` (`self.Face`) "Vinny_RightBrow_Mad") (+ Vinny_RightBrow_Mad (`KismetMathLibrary.RandomFloatInRange` -0.1 0.1)) (`self.Alpha`)) true)
      (`SkeletalMeshComponent.SetMorphTarget` (`self.Face`) "Vinny_LeftBrow_Sad" (`KismetMathLibrary.Lerp` (`SkeletalMeshComponent.GetMorphTarget` (`self.Face`) "Vinny_LeftBrow_Sad") Vinny_LeftBrow_Sad (`self.Alpha`)) true)
      (`SkeletalMeshComponent.SetMorphTarget` (`self.Face`) "Vinny_RightBrow_Sad" (`KismetMathLibrary.Lerp` (`SkeletalMeshComponent.GetMorphTarget` (`self.Face`) "Vinny_RightBrow_Sad") Vinny_RightBrow_Sad (`self.Alpha`)) true)
      (`SkeletalMeshComponent.SetMorphTarget` (`self.Face`) "Vinny_Mouth_Smile" (`KismetMathLibrary.Lerp` (`SkeletalMeshComponent.GetMorphTarget` (`self.Face`) "Vinny_Mouth_Smile") Vinny_Mouth_Smile (`self.Alpha`)) true)
      (`SkeletalMeshComponent.SetMorphTarget` (`self.Face`) "Vinny_Mouth_Frown" (`KismetMathLibrary.Lerp` (`SkeletalMeshComponent.GetMorphTarget` (`self.Face`) "Vinny_Mouth_Frown") Vinny_Mouth_Frown (`self.Alpha`)) true)
      (`SkeletalMeshComponent.SetMorphTarget` (`self.Face`) "Vinny_Infection" (`KismetMathLibrary.Lerp` (`SkeletalMeshComponent.GetMorphTarget` (`self.Face`) "Vinny_Infection") (+ Vinny_Infection (`KismetMathLibrary.RandomFloatInRange` -0.2 0.2)) (`self.Alpha`)) true)
      (`SkeletalMeshComponent.SetMorphTarget` (`self.Face`) "Vinny_Creep" (`KismetMathLibrary.Lerp` (`SkeletalMeshComponent.GetMorphTarget` (`self.Face`) "Vinny_Creep") Vinny_Creep (`self.Alpha`)) true)
      (`SkeletalMeshComponent.SetMorphTarget` (`self.Face`) "Toothy_Smile" (`KismetMathLibrary.Lerp` (`SkeletalMeshComponent.GetMorphTarget` (`self.Face`) "Toothy_Smile") Toothy_Smile (`self.Alpha`)) true)
      (`SkeletalMeshComponent.SetMorphTarget` (`self.Face`) "Tooth_Scowl" (`KismetMathLibrary.Lerp` (`SkeletalMeshComponent.GetMorphTarget` (`self.Face`) "Tooth_Scowl") Tooth_Scowl (`self.Alpha`)) true)
      (`SkeletalMeshComponent.SetMorphTarget` (`self.Face`) "Right_Smirk" (`KismetMathLibrary.Lerp` (`SkeletalMeshComponent.GetMorphTarget` (`self.Face`) "Right_Smirk") (+ Right_Smirk (`KismetMathLibrary.RandomFloatInRange` -0.1 0.1)) (`self.Alpha`)) true)
      (`SkeletalMeshComponent.SetMorphTarget` (`self.Face`) "Left_Smirk" (`KismetMathLibrary.Lerp` (`SkeletalMeshComponent.GetMorphTarget` (`self.Face`) "Left_Smirk") (+ Left_Smirk (`KismetMathLibrary.RandomFloatInRange` -0.1 0.1)) (`self.Alpha`)) true)
      (`SkeletalMeshComponent.SetMorphTarget` (`self.Face`) "Right_Eye_Wide" (`KismetMathLibrary.Lerp` (`SkeletalMeshComponent.GetMorphTarget` (`self.Face`) "Right_Eye_Wide") (+ Right_Eye_Wide (`KismetMathLibrary.RandomFloatInRange` -0.1 0.1)) (`self.Alpha`)) true)
      (`SkeletalMeshComponent.SetMorphTarget` (`self.Face`) "Left_Eye_Wide" (`KismetMathLibrary.Lerp` (`SkeletalMeshComponent.GetMorphTarget` (`self.Face`) "Left_Eye_Wide") (+ Left_Eye_Wide (`KismetMathLibrary.RandomFloatInRange` -0.1 0.1)) (`self.Alpha`)) true)
      (`SkeletalMeshComponent.SetMorphTarget` (`self.Face`) "Melt" (`KismetMathLibrary.Lerp` (`SkeletalMeshComponent.GetMorphTarget` (`self.Face`) "Melt") Melt (`self.Alpha`)) true))))

(fn `ExitCarAnimation`
  (bind _asmanny_animation_blueprint (cast `/Game/Animations/MannyAnimationBlueprint` (`SkeletalMeshComponent.GetAnimInstance` (`self.Mesh`))))
  (set `/Game/Animations/MannyAnimationBlueprint.IsWalking` false _asmanny_animation_blueprint)
  (set `/Game/Animations/MannyAnimationBlueprint.GetInCar` false _asmanny_animation_blueprint)
  (set `/Game/Animations/MannyAnimationBlueprint.ExitCar` true _asmanny_animation_blueprint)
  (set `/Game/Animations/MannyAnimationBlueprint.GrabItem` false _asmanny_animation_blueprint)
  (set `/Game/Animations/MannyAnimationBlueprint.StabPlayer` false _asmanny_animation_blueprint)
  (set `/Game/Animations/MannyAnimationBlueprint.IsStaring` false _asmanny_animation_blueprint))

(fn `GetInCarAnimation`
  (bind _asmanny_animation_blueprint (cast `/Game/Animations/MannyAnimationBlueprint` (`SkeletalMeshComponent.GetAnimInstance` (`self.Mesh`))))
  (set `/Game/Animations/MannyAnimationBlueprint.IsWalking` false _asmanny_animation_blueprint)
  (set `/Game/Animations/MannyAnimationBlueprint.GetInCar` true _asmanny_animation_blueprint)
  (set `/Game/Animations/MannyAnimationBlueprint.ExitCar` false _asmanny_animation_blueprint)
  (set `/Game/Animations/MannyAnimationBlueprint.GrabItem` false _asmanny_animation_blueprint)
  (set `/Game/Animations/MannyAnimationBlueprint.StabPlayer` false _asmanny_animation_blueprint)
  (set `/Game/Animations/MannyAnimationBlueprint.IsStaring` false _asmanny_animation_blueprint))

(fn `Grabbing Item Animation`
  (bind _asmanny_animation_blueprint (cast `/Game/Animations/MannyAnimationBlueprint` (`SkeletalMeshComponent.GetAnimInstance` (`self.Mesh`))))
  (set `/Game/Animations/MannyAnimationBlueprint.IsWalking` false _asmanny_animation_blueprint)
  (set `/Game/Animations/MannyAnimationBlueprint.GetInCar` false _asmanny_animation_blueprint)
  (set `/Game/Animations/MannyAnimationBlueprint.ExitCar` false _asmanny_animation_blueprint)
  (set `/Game/Animations/MannyAnimationBlueprint.GrabItem` true _asmanny_animation_blueprint)
  (set `/Game/Animations/MannyAnimationBlueprint.StabPlayer` false _asmanny_animation_blueprint)
  (set `/Game/Animations/MannyAnimationBlueprint.IsStaring` false _asmanny_animation_blueprint))

(fn `IdleAnimation`
  (bind _asmanny_animation_blueprint (cast `/Game/Animations/MannyAnimationBlueprint` (`SkeletalMeshComponent.GetAnimInstance` (`self.Mesh`))))
  (set `/Game/Animations/MannyAnimationBlueprint.IsWalking` false _asmanny_animation_blueprint)
  (set `/Game/Animations/MannyAnimationBlueprint.GetInCar` false _asmanny_animation_blueprint)
  (set `/Game/Animations/MannyAnimationBlueprint.ExitCar` false _asmanny_animation_blueprint)
  (set `/Game/Animations/MannyAnimationBlueprint.GrabItem` false _asmanny_animation_blueprint)
  (set `/Game/Animations/MannyAnimationBlueprint.StabPlayer` false _asmanny_animation_blueprint)
  (set `/Game/Animations/MannyAnimationBlueprint.IsStaring` false _asmanny_animation_blueprint))

(fn `Stabbing Animation`
  (bind _asmanny_animation_blueprint (cast `/Game/Animations/MannyAnimationBlueprint` (`SkeletalMeshComponent.GetAnimInstance` (`self.Mesh`))))
  (set `/Game/Animations/MannyAnimationBlueprint.IsWalking` false _asmanny_animation_blueprint)
  (set `/Game/Animations/MannyAnimationBlueprint.GetInCar` false _asmanny_animation_blueprint)
  (set `/Game/Animations/MannyAnimationBlueprint.ExitCar` false _asmanny_animation_blueprint)
  (set `/Game/Animations/MannyAnimationBlueprint.GrabItem` false _asmanny_animation_blueprint)
  (set `/Game/Animations/MannyAnimationBlueprint.StabPlayer` true _asmanny_animation_blueprint)
  (set `/Game/Animations/MannyAnimationBlueprint.IsStaring` false _asmanny_animation_blueprint))

(fn `Staring Animation`
  (bind _asmanny_animation_blueprint (cast `/Game/Animations/MannyAnimationBlueprint` (`SkeletalMeshComponent.GetAnimInstance` (`self.Mesh`))))
  (set `/Game/Animations/MannyAnimationBlueprint.IsWalking` false _asmanny_animation_blueprint)
  (set `/Game/Animations/MannyAnimationBlueprint.GetInCar` false _asmanny_animation_blueprint)
  (set `/Game/Animations/MannyAnimationBlueprint.ExitCar` false _asmanny_animation_blueprint)
  (set `/Game/Animations/MannyAnimationBlueprint.GrabItem` false _asmanny_animation_blueprint)
  (set `/Game/Animations/MannyAnimationBlueprint.StabPlayer` false _asmanny_animation_blueprint)
  (set `/Game/Animations/MannyAnimationBlueprint.IsStaring` true _asmanny_animation_blueprint))

(fn `UserConstructionScript`
  (`SkinnedMeshComponent.SetLeaderPoseComponent` (`self.Legs`) (`self.Body`) false false)
  (`SkinnedMeshComponent.SetLeaderPoseComponent` (`self.Feet`) (`self.Body`) false false)
  (`SkinnedMeshComponent.SetLeaderPoseComponent` (`self.Face`) (`self.Body`) false false)
  (`SkinnedMeshComponent.SetLeaderPoseComponent` (`self.Torso`) (`self.Body`) false false))