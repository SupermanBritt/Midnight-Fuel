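; A grabbable soda actor that can be delivered to a customer waiting at a window.
; It stores its starting transform and, on overlapping the OutOfBoundsBox, releases the grab and resets there, toggling physics around the move.
; While a NormalCustomer2 found by class lookup is AtWindow, grabbing the soda calls its Disappear, and Deliver calls GetInCar and destroys the soda.
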(event `self.ReceiveBeginPlay`
  (set `self.Original Position` (`self.GetTransform`)))

(event `Reset Position`
  (bind _soda (`self.Soda`))
  (`/Game/VRTemplate/Blueprints/GrabComponent.TryRelease` (`self.GrabComponent`))
  (`PrimitiveComponent.SetSimulatePhysics` _soda false)
  (`self.K2_SetActorTransform` (`self.Original Position`))
  (`PrimitiveComponent.SetSimulatePhysics` _soda true))

(event `self.Soda.OnComponentBeginOverlap`
  (params (OverlappedComponent :type "PrimitiveComponent Object Reference") (OtherActor :type "Actor Object Reference") (OtherComp :type "PrimitiveComponent Object Reference") (OtherBodyIndex :type Integer) (bFromSweep :type Boolean) (SweepResult :type "HitResult Structure (by ref)"))
  (bind _returnvalue (`GameplayStatics.GetActorOfClass` "/Game/Blueprints/OutOfBoundsBox.OutOfBoundsBox_C"))
  (if (== _returnvalue OtherActor)
    (`self.Reset Position`)))

(event `Deliver`
  (bind _returnvalue (`GameplayStatics.GetActorOfClass` "/Game/Blueprints/NormalCustomer2.NormalCustomer2_C"))
  (if (`/Game/Blueprints/NormalCustomer2.AtWindow` _returnvalue)
    (`/Game/Blueprints/NormalCustomer2.Get In Car` _returnvalue)
    (`self.K2_DestroyActor`)))

(event `self.GrabComponent.OnGrabbed`
  (bind _returnvalue (`GameplayStatics.GetActorOfClass` "/Game/Blueprints/NormalCustomer2.NormalCustomer2_C"))
  (if (`/Game/Blueprints/NormalCustomer2.AtWindow` _returnvalue)
    (`/Game/Blueprints/NormalCustomer2.Disappear` _returnvalue)))

(fn `UserConstructionScript`)