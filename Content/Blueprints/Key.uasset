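; Key actor with a physics-simulated component that returns to its starting spot when it leaves the play area.
; It records its transform at BeginPlay and calls ResetPosition when the Key component overlaps the OutOfBoundsBox found by GetActorOfClass, so only that one instance triggers a reset.
; ResetPosition switches physics simulation off, restores the saved transform, then switches simulation back on.
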(event `self.ReceiveBeginPlay`
  (set `self.Original Position` (`self.GetTransform`)))

(event `Reset Position`
  (bind _key (`self.Key`))
  (`PrimitiveComponent.SetSimulatePhysics` _key false)
  (`self.K2_SetActorTransform` (`self.Original Position`))
  (`PrimitiveComponent.SetSimulatePhysics` _key true))

(event `self.Key.OnComponentBeginOverlap`
  (params (OverlappedComponent :type "PrimitiveComponent Object Reference") (OtherActor :type "Actor Object Reference") (OtherComp :type "PrimitiveComponent Object Reference") (OtherBodyIndex :type Integer) (bFromSweep :type Boolean) (SweepResult :type "HitResult Structure (by ref)"))
  (bind _returnvalue (`GameplayStatics.GetActorOfClass` "/Game/Blueprints/OutOfBoundsBox.OutOfBoundsBox_C"))
  (if (== _returnvalue OtherActor)
    (`self.Reset Position`)))

(fn `UserConstructionScript`)