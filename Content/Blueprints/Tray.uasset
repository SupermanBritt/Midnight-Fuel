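; Grabbable sliding tray that delivers one of four recognized items when dragged to its negative X limit.
; Box overlaps track the item by component name, and Tick calls Deliver on the first actor of the matching class.
; Tick also locks rotation, Y and Z and clamps X travel, but only once Y or Z drifts.
; A timeline-driven PullTrayOut event slides it out, and right-hand grabs rotate it half a turn.
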(event `self.GrabComponent.OnGrabbed`
  (if (`|EnumEquality` (`/Game/VRTemplate/Blueprints/GrabComponent.GetHeldByHand` (`self.GrabComponent`)) "Right")
    (`self.K2_SetActorRotation` (`KismetMathLibrary.ComposeRotators` (`self.K2_GetActorRotation`) (struct :`Roll` 180.0)) true)))

(event `self.GrabComponent.OnDropped`
  (`self.K2_SetActorRotation` (struct)))

(event `Pull Tray Out`
  (set `self.CurrentPosition` (`self.K2_GetActorLocation`))
  (bind (_direction _alpha) (`Timeline|Timeline`)
    (:`Update`
      (`self.K2_SetActorLocation` (`KismetMathLibrary.VLerp` (`self.CurrentPosition`) (- (`self.OriginalPosition`) (25.0 0.0 0.0)) _alpha)))))

(event `self.Box.OnComponentBeginOverlap`
  (params (OverlappedComponent :type "PrimitiveComponent Object Reference") (OtherActor :type "Actor Object Reference") (OtherComp :type "PrimitiveComponent Object Reference") (OtherBodyIndex :type Integer) (bFromSweep :type Boolean) (SweepResult :type "HitResult Structure (by ref)"))
  (bind _returnvalue (`KismetSystemLibrary.GetObjectName` OtherComp))
  (set `self.Tray Item` _returnvalue)
  (if (or (`KismetStringLibrary.EqualEqual_StrStr` _returnvalue "Phonebook") (`KismetStringLibrary.EqualEqual_StrStr` _returnvalue "Chips") (`KismetStringLibrary.EqualEqual_StrStr` _returnvalue "Soda") (`KismetStringLibrary.EqualEqual_StrStr` _returnvalue "Tooth"))
    (set `self.InTray` true)))

(event `self.Box.OnComponentEndOverlap`
  (params (OverlappedComponent :type "PrimitiveComponent Object Reference") (OtherActor :type "Actor Object Reference") (OtherComp :type "PrimitiveComponent Object Reference") (OtherBodyIndex :type Integer))
  (bind _returnvalue (`KismetSystemLibrary.GetObjectName` OtherComp))
  (if (or (`KismetStringLibrary.EqualEqual_StrStr` _returnvalue "Phonebook") (`KismetStringLibrary.EqualEqual_StrStr` _returnvalue "Chips") (`KismetStringLibrary.EqualEqual_StrStr` _returnvalue "Soda") (`KismetStringLibrary.EqualEqual_StrStr` _returnvalue "Tooth"))
    (set `self.InTray` false)))

(event `self.ReceiveBeginPlay`
  (set `self.OriginalPosition` (`self.K2_GetActorLocation`)))

(event `self.ReceiveTick`
  (params (DeltaSeconds :type "Float (single-precision)"))
  (bind _returnvalue (- (.x (`self.OriginalPosition`)) (.x (`self.NewPosition`))))
  (bind _returnvalue_2 (> _returnvalue 25.0))
  (set `self.NewPosition` (`self.K2_GetActorLocation`))
  (if (or (!= (.y (`self.OriginalPosition`)) (.y (`self.NewPosition`))) (!= (.z (`self.OriginalPosition`)) (.z (`self.NewPosition`))))
    (`self.K2_SetActorLocation` (`KismetMathLibrary.MakeVector` (.x (`self.NewPosition`)) (.y (`self.OriginalPosition`)) (.z (`self.OriginalPosition`))))
    (`self.K2_SetActorRotation` (struct))
    (if _returnvalue_2
      (`self.K2_SetActorLocation` (`KismetMathLibrary.MakeVector` (- (.x (`self.OriginalPosition`)) 25.0) (.y (`self.OriginalPosition`)) (.z (`self.OriginalPosition`))))
      (if (and _returnvalue_2 (`self.InTray`))
        (switch `string` (`self.Tray Item`)
          (:`Phonebook`
            (bind _returnvalue_3 (`GameplayStatics.GetActorOfClass` "/Game/Blueprints/Phonebook.Phonebook_C"))
            (`/Game/Blueprints/Phonebook.Deliver` _returnvalue_3))
          (:`Chips`
            (bind _returnvalue_4 (`GameplayStatics.GetActorOfClass` "/Game/Blueprints/Chips.Chips_C"))
            (`/Game/Blueprints/Chips.Deliver` _returnvalue_4))
          (:`Soda`
            (bind _returnvalue_5 (`GameplayStatics.GetActorOfClass` "/Game/Blueprints/Soda.Soda_C"))
            (`/Game/Blueprints/Soda.Deliver` _returnvalue_5))
          (:`Tooth`
            (bind _returnvalue_6 (`GameplayStatics.GetActorOfClass` "/Game/Blueprints/Tooth.Tooth_C"))
            (`/Game/Blueprints/Tooth.Deliver` _returnvalue_6))))
      (elif (< _returnvalue -25.0)
        (`self.K2_SetActorLocation` (`KismetMathLibrary.MakeVector` (+ (.x (`self.OriginalPosition`)) 25.0) (.y (`self.OriginalPosition`)) (.z (`self.OriginalPosition`))))))))

(fn `UserConstructionScript`)