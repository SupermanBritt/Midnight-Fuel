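; NormalCustomer1 is a customer actor that travels from its car to a service window and back along the spline of a CustomerPath actor found at BeginPlay.
; GetOutofCar plays a timeline that lerps distance along the spline to set location and rotation, then flags AtWindow.
; GetInCar reverses a second timeline along the same path, then flags ItemDelivered, teleports to the original position and calls CallFirstCustomer.
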(event `self.ReceiveBeginPlay`
  (set `self.Original Position` (`self.K2_GetActorLocation`))
  (bind _returnvalue (`GameplayStatics.GetActorOfClass` "/Game/Blueprints/CustomerPath.CustomerPath_C"))
  (set `self.CustomerPath` _returnvalue))

(event `Get Out of Car`
  (bind (_direction _alpha) (`Timeline|Timeline`)
    (:`Update`
      (`self.K2_SetActorLocationAndRotation` (.location (`SplineComponent.GetTransformAtDistanceAlongSpline` (`/Game/Blueprints/CustomerPath.Spline` (`self.CustomerPath`)) (`KismetMathLibrary.Lerp` 0.0 (`SplineComponent.GetSplineLength` (`/Game/Blueprints/CustomerPath.Spline` (`self.CustomerPath`))) _alpha) "World" false)) (.rotation (`SplineComponent.GetTransformAtDistanceAlongSpline` (`/Game/Blueprints/CustomerPath.Spline` (`self.CustomerPath`)) (`KismetMathLibrary.Lerp` 0.0 (`SplineComponent.GetSplineLength` (`/Game/Blueprints/CustomerPath.Spline` (`self.CustomerPath`))) _alpha) "World" false))))
    (:`Finished`
      (set `self.AtWindow` true))))

(event `Get In Car`
  (bind (_direction _alpha) (`Timeline|Timeline_0` :!via `ReverseFromEnd`)
    (:`Update`
      (`self.K2_SetActorLocationAndRotation` (.location (`SplineComponent.GetTransformAtDistanceAlongSpline` (`/Game/Blueprints/CustomerPath.Spline` (`self.CustomerPath`)) (`KismetMathLibrary.Lerp` 0.0 (`SplineComponent.GetSplineLength` (`/Game/Blueprints/CustomerPath.Spline` (`self.CustomerPath`))) _alpha) "World" false)) (.rotation (`SplineComponent.GetTransformAtDistanceAlongSpline` (`/Game/Blueprints/CustomerPath.Spline` (`self.CustomerPath`)) (`KismetMathLibrary.Lerp` 0.0 (`SplineComponent.GetSplineLength` (`/Game/Blueprints/CustomerPath.Spline` (`self.CustomerPath`))) _alpha) "World" false))))
    (:`Finished`
      (set `self.ItemDelivered` true)
      (`self.K2_TeleportTo` (`self.Original Position`))
      (`self.First Customer`))))

(fn `UserConstructionScript`)