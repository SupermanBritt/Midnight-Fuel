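; BP_ceilling_Fan is a gas station ceiling fan with a point light that can be switched on and off.
; Tick spins the fan mesh around yaw by FanSpeed each frame, without delta-time scaling, so its speed depends on frame rate; BeginPlay applies the same rotation once.
; The TurnOnLights and TurnOffLights events toggle the light by setting its intensity to a fixed level or zero.
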(event `Turn Off Lights`
  (`LightComponent.SetIntensity` (`self.PointLight`) 0.0))

(event `Turn On Lights`
  (`LightComponent.SetIntensity` (`self.PointLight`) 1300.0))

(event `self.ReceiveTick`
  (params (DeltaSeconds :type "Float (single-precision)"))
  (`SceneComponent.K2_AddLocalRotation` (`self.SM_Ceiling_Fan_Cylinder_005`) (`KismetMathLibrary.MakeRotator` 0.0 0.0 (`self.Fan speed`)) false false :!label _label))

(event `self.ReceiveBeginPlay`
  (goto _label))

(fn `UserConstructionScript`)